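; BP_NovaBomb is the actor for the player's Nova Bomb super, which kills basic enemies on contact.
; On overlap it casts the other actor to BP_BasicEnemy, prints a debug message and destroys that enemy outright, while the bomb itself carries on.
; Tick accumulates elapsed time and destroys the bomb once KillTime is reached, unless IsPersistent is set.
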(event `self.ReceiveBeginPlay`)

(event `self.ReceiveActorBeginOverlap`
  (params (OtherActor :type "Actor Object Reference"))
  ; If an enemy comes into contact with the Nova Bomb, kill them.
  (bind _asbp_basic_enemy (cast `/Game/Enemies/BP_BasicEnemy` OtherActor))
  (`KismetSystemLibrary.PrintString` "Enemy Killed")
  (`self.K2_DestroyActor` _asbp_basic_enemy))

(event `self.ReceiveTick`
  (params (DeltaSeconds :type "Float (single-precision)"))
  ; Destroy the Nova Bomb after its kill time has been reached.
  (if (`self.bIsPersistent`)
    _
    (elif (< (`self.SecondsPassed`) (`self.KillTime`))
      (set `self.SecondsPassed` (+ (`self.SecondsPassed`) DeltaSeconds))
      (else
        (`self.K2_DestroyActor`)))))

(fn `UserConstructionScript`)