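; Player character Blueprint with Enhanced Input look, move and jump, plus a subclass-based Super ability.
; Casting a Super launches the player upward; Tick fires it once vertical velocity turns downward and re-arms it on the ground.
; Solar spawns a symmetric row of forward-flying blades, while Void spawns a Nova Bomb ahead.
; Subclass is temporarily hardcoded to Solar on BeginPlay, pending a menu.
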(event `self.ReceiveBeginPlay`
  ; Assign the player's input mapping context.
  (bind _returnvalue (`InputDeviceLibrary.GetPlayerControllerFromInputDevice` (struct)))
  (`EnhancedInputSubsystemInterface.AddMappingContext` (pcsubsystem `EnhancedInputLocalPlayerSubsystem` _returnvalue) "/Game/Player/Input/IMC_PlayerInput.IMC_PlayerInput" 0 (struct))
  ; Temporary Subclass assignment (Will later be replaced with a menu.)
  (set `self.Subclass` "NewEnumerator0"))

(event `self.ReceiveTick`
  (params (DeltaSeconds :type "Float (single-precision)"))
  (`|ExecutionSequence`
    (:`then_0`
      ; Active a Super when the apex of the jump has been reached.
      (if (`self.bHasSupered`)
        (bind _returnvalue (`PrimitiveComponent.GetPhysicsLinearVelocity` (`self.CapsuleComponent`) "None"))
        (if (<= (.z _returnvalue) -1.0)
          (switch `/Game/Player/PlayerSubclass` (`self.Subclass`)
            (:`NewEnumerator0`
              (`self.ActivateBladeBarrage`))
            (:`NewEnumerator1`
              (`self.activateNovaBomb`))))))
    (:`then_1`
      ; Re-Enable the super when the player has hit the ground.
      (if (not (`NavMovementComponent.IsFalling` (`self.CharacterMovement`)))
        (set `self.bCanSuper` true)))))

(event `EnhancedInput|/Game/Player/Input/IA_Super`
  (params (ActionValue :type Boolean) (ElapsedSeconds :type "Float (double-precision)") (TriggeredSeconds :type "Float (double-precision)") (InputAction :type "InputAction Object Reference" :default "/Game/Player/Input/IA_Super.IA_Super"))
  (:`Started`
    (if (and (`self.bCanSuper`) (not (`self.bHasSupered`)))
      (`self.LaunchCharacter` (`KismetMathLibrary.MakeVector` 0.0 0.0 (`KismetMathLibrary.Conv_IntToDouble` (`self.JumpForce`))))
      (set `self.bHasSupered` true)
      (set `self.bCanSuper` false)
      (`KismetSystemLibrary.PrintString` "Super Cast"))))

(event `EnhancedInput|/Game/Player/Input/IA_Look`
  (params (ActionValue :type "Vector2D Structure") (ElapsedSeconds :type "Float (double-precision)") (TriggeredSeconds :type "Float (double-precision)") (InputAction :type "InputAction Object Reference" :default "/Game/Player/Input/IA_Look.IA_Look"))
  (:`Triggered`
    ; Player look input.
    (`self.AddControllerYawInput` ActionValue_X)
    (`self.AddControllerPitchInput` (* ActionValue_Y -1.0))))

(event `EnhancedInput|/Game/Player/Input/IA_Move`
  (params (ActionValue :type "Vector2D Structure") (ElapsedSeconds :type "Float (double-precision)") (TriggeredSeconds :type "Float (double-precision)") (InputAction :type "InputAction Object Reference" :default "/Game/Player/Input/IA_Move.IA_Move"))
  (:`Triggered`
    ; Player move input.
    (`self.AddMovementInput` (`KismetMathLibrary.GetForwardVector` (`self.GetControlRotation`)) ActionValue_Y)
    (`self.AddMovementInput` (`KismetMathLibrary.GetRightVector` (`self.GetControlRotation`)) ActionValue_X)))

(event `EnhancedInput|/Game/Player/Input/IA_Jump`
  (params (ActionValue :type Boolean) (ElapsedSeconds :type "Float (double-precision)") (TriggeredSeconds :type "Float (double-precision)") (InputAction :type "InputAction Object Reference" :default "/Game/Player/Input/IA_Jump.IA_Jump"))
  (:`Triggered`
    ; Player jump input.
    (if (not (`NavMovementComponent.IsFalling` (`self.CharacterMovement`)))
      (`self.LaunchCharacter` (0.0 0.0 500.0)))))

(fn `ActivateBladeBarrage`
  (locals (NewLocalVar :type Integer))
  (for _index (range (`self.bladesToSpawn`))
    (if (== _index 0)
      (`self.SpawnBlade` (+ (`self.K2_GetActorLocation`) (* (`SceneComponent.GetForwardVector` (`self.CapsuleComponent`)) 300.0)) (`self.K2_GetActorRotation`))
      (else
        (`self.SpawnBlade` (+ (`self.K2_GetActorLocation`) (* (`SceneComponent.GetForwardVector` (`self.CapsuleComponent`)) 300.0) (* (`self.GetActorRightVector`) (* (`self.bladesSpacing`) _index))) (`self.K2_GetActorRotation`))
        (`self.SpawnBlade` (+ (`self.K2_GetActorLocation`) (* (`SceneComponent.GetForwardVector` (`self.CapsuleComponent`)) 300.0) (* (`self.GetActorRightVector`) (* (`self.bladesSpacing`) _index) -1.0)) (`self.K2_GetActorRotation`)))))
  (set `self.bHasSupered` false))

(fn `activateNovaBomb`
  (locals (NewLocalVar :type Integer))
  (`self.SpawnNovaBomb` (+ (`self.K2_GetActorLocation`) (* (`SceneComponent.GetForwardVector` (`self.CapsuleComponent`)) 1000.0)) (`self.K2_GetActorRotation`))
  (set `self.bHasSupered` false))

(fn `SpawnBlade`
  (params (SpawnPos :type "Vector Structure") (spawnRot :type "Rotator Structure"))
  (returns (BladeRef :type "Object Object Reference"))
  (bind _returnvalue (`|SpawnActorFromClass` "/Game/Player/Supers/Blade_Barrage/BP_Blade.BP_Blade_C" (`KismetMathLibrary.MakeTransform` SpawnPos spawnRot) "Undefined" "MultiplyWithRoot" null null))
  (`PrimitiveComponent.SetPhysicsLinearVelocity` (`/Game/Player/Supers/Blade_Barrage/BP_Blade.Plane` _returnvalue) (* (`SceneComponent.GetForwardVector` (`self.CapsuleComponent`)) (`self.bladeSpeed`)) false "None")
  (return _returnvalue))

(fn `SpawnNovaBomb`
  (params (SpawnPos :type "Vector Structure") (spawnRot :type "Rotator Structure"))
  (returns (NovaBombRef :type "Object Object Reference"))
  (bind _returnvalue (`|SpawnActorFromClass` "/Game/Player/Supers/Nova_Bomb/BP_NovaBomb.BP_NovaBomb_C" (`KismetMathLibrary.MakeTransform` SpawnPos spawnRot) "Undefined" "MultiplyWithRoot" null null))
  (return _returnvalue))

(fn `UserConstructionScript`)